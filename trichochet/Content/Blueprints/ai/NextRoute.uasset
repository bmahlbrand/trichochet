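; Behavior Tree task meant to point an AI's TargetPoint blackboard key at the waypoint for its current Route index.
; On execute it wraps Route to zero at MaxRoutes and gathers all Waypoint actors.
; The loop matching Waypoint Position to Route and writing its location is disconnected, so TargetPoint is never updated.
; FinishExecute, set to report failure, sits in that unreached branch, so the task never finishes.
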(event EventReceiveExecute
  (params (OwnerActor :type Actor%20Object%20Reference))
  (bind _route (Variables|Default|GetRoute))
  ;[1 1 1] Update TargetPoint to NextRoute
  (if (>= (Class|BTFunctionLibrary|GetBlackboardValueasInt _route) (Variables|Default|GetMaxRoutes))
    (Class|BTFunctionLibrary|SetBlackboardValueasInt _route))
  (bind _outactors (Actor|GetAllActorsOfClass "/Game/Blueprints/ai/Waypoint.Waypoint_C")))