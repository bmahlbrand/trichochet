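; Behavior tree task that moves the Bot controller's pawn to within range of the TargetToFollow blackboard actor.
; It caches the Bot reference, runs AI MoveTo, then on success spawns an explosion at the target and finishes.
; A failed move never finishes the task.
; A separate SetWalkspeed function, not called here, sets the player character's walk speed rather than the bot's.
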(event EventReceiveExecute
  (params (OwnerActor :type Actor%20Object%20Reference))
  (bind _targettofollow (Variables|Default|GetTargetToFollow))
  (bind _returnvalue (AI|BehaviorTree|GetBlackboardValueasActor _targettofollow))
  (if (Utilities|IsValid (Variables|Default|GetAI_CON_REF))
    _
    (else
      (bind _asbot (Utilities|Casting|CastToBot OwnerActor))
      (Variables|Default|SetAI_CON_REF _asbot)))
  (AI|AIMoveTo (Pawn|GetControlledPawn (Variables|Default|GetAI_CON_Ref)) "0, 0, 0" _returnvalue 5e+02 false
    (:OnSuccess
      (Effects|SpawnEmitteratLocation "/Game/Lesson2/Effects/P_Explosion_Orange2.P_Explosion_Orange2" (Transformation|GetActorLocation _returnvalue) "0.000000, 0,0.000000")
      (AI|BehaviorTree|FinishExecute true))))

(fn SetWalkspeed
  (bind _ascharacter_movement_component (Utilities|Casting|CastToCharacterMovementComponent (Pawn|GetMovementComponent (Game|GetPlayerCharacter 0))))
  (Variables|/Script/Engine.CharacterMovementComponent|SetMaxWalkSpeed _ascharacter_movement_component 6e+02))