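; CloseEnough is a behavior tree decorator condition for the Bot AI that gates behavior on distance to a follow target.
; It casts the owner to Bot, then measures the distance from its controlled pawn to the TargetToFollow blackboard actor.
; Despite the name, it passes when that distance is at least AcceptableDistance, meaning the bot is not yet close enough.
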(fn PerformConditionCheck
  (params (OwnerActor :type Actor%20Object%20Reference))
  (bind _asbot (Utilities|Casting|CastToBot OwnerActor))
  (Variables|Default|SetAI_CON_Ref _asbot)
  (return (>= (Math|Vector|VectorLength (- (Transformation|GetActorLocation (AI|BehaviorTree|GetBlackboardValueasActor (Variables|Default|GetTargetToFollow))) (Transformation|GetActorLocation (Pawn|GetControlledPawn (Variables|Default|GetAI_CON_Ref))))) (Variables|Default|GetAcceptableDistance))))