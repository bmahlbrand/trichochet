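; Behavior tree node that gives bots aggro by finding a visible target around their pawn.
; Each tick it sphere-traces a wide radius for configured object types, ignoring all BotChar actors, using a lazily cached Bot controller.
; A debug-drawn Camera-channel line trace tests sight to each hit, setting TargetToFollow and TargetLocation, or clearing only TargetToFollow when blocked.
; The last hit processed decides the target.
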(event EventTick
  (params (OwnerActor :type Actor%20Object%20Reference) (DeltaSeconds :type Float%20%28single-precision%29))
  (if (Utilities|IsValid (Variables|Default|GetBot_CON_Ref))
    _
    (else
      (bind _asbot (Utilities|Casting|CastToBot OwnerActor))
      (bind _output_get (Variables|Default|SetBot_CON_Ref _asbot))))
  (bind _outactors (Actor|GetAllActorsOfClass "/Game/Blueprints/ai/BotChar.BotChar_C"))
  (Variables|Default|SetMyLocation (Transformation|GetActorLocation (Pawn|GetControlledPawn _output_get)))
  (bind _outhits (Collision|MultiSphereTraceForObjects (Transformation|GetActorLocation (Pawn|GetControlledPawn _output_get)) (+ (Transformation|GetActorLocation (Pawn|GetControlledPawn _output_get)) "0, 0,15.000000") 1.5e+03 (Variables|Default|GetDesiredObjectTypes) false _outactors "None"))
  (bind _array_element (Utilities|Array|ForEachLoopwithBreak _outhits)
    (:LoopBody
      (bind _outhit (Collision|LineTraceByChannel (Variables|Default|GetMyLocation) (Transformation|GetActorLocation (.HitActor (Collision|BreakHitResult _array_element))) "TraceTypeQuery2" false _outactors "ForDuration"))
      (if (== (.HitActor (Collision|BreakHitResult _outhit)) (.HitActor (Collision|BreakHitResult _array_element)))
        (Class|BTFunctionLibrary|SetBlackboardValueasObject (Variables|Default|GetTargetToFollow) (.HitActor (Collision|BreakHitResult _outhit)))
        (AI|BehaviorTree|SetBlackboardValueasVector (Variables|Default|GetTargetLocation) (Transformation|GetActorLocation (.HitActor (Collision|BreakHitResult _outhit))))
        (else
          (Class|BTFunctionLibrary|SetBlackboardValueasObject (Variables|Default|GetTargetToFollow)))))))