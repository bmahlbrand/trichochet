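; NextRoute is a Behavior Tree task that points the AI's TargetPoint at the waypoint for its current route index.
; It resets the Route blackboard value to zero once it reaches MaxRoutes, but never increments it.
; It then scans all Waypoint actors and writes the location of the one whose Position matches Route to TargetPoint.
; The task finishes reporting failure, even when a match is found.
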(event EventReceiveExecute
  (params (OwnerActor :type Actor%20Object%20Reference))
  (bind _route (Variables|Default|GetRoute))
  ;[1 1 1] Update TargetPoint to NextRoute
  (if (>= (Class|BTFunctionLibrary|GetBlackboardValueasInt _route) (Variables|Default|GetMaxRoutes))
    (Class|BTFunctionLibrary|SetBlackboardValueasInt _route))
  (bind _outactors (Actor|GetAllActorsOfClass "/Game/Blueprints/ai/Waypoint.Waypoint_C"))
  (bind _array_element (Utilities|Array|ForEachLoopwithBreak _outactors)
    (:LoopBody
      (bind _aswaypoint (Utilities|Casting|CastToWaypoint _array_element))
      (if (== (Variables|/Game/Blueprints/ai/Waypoint.Waypoint_C|GetPosition _aswaypoint) (Class|BTFunctionLibrary|GetBlackboardValueasInt (Variables|Default|GetRoute)))
        (AI|BehaviorTree|SetBlackboardValueasVector (Variables|Default|GetTargetPoint) (Transformation|GetActorLocation _aswaypoint))))
    (:Completed
      (AI|BehaviorTree|FinishExecute false))))