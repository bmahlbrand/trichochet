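; Game mode for a two-player match that registers each joining player and starts play through ready checks.
; It spawns two TR_GameStatus scoreboards on the first game, then resets scores and a looping countdown timer.
; A fall awards the opponent a point, teleports both players to start positions and begins a new round.
; The Rounds OnRep restarts the game at ten, as does agreement from both players.
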(event Custom|Begin%20ROund
  ;[1 1 1] Setup New Round
  (bind _output_get (Variables|Default|SetRoundTime 300))
  (Default|UpdateRoundTime (Variables|Default|GetScoreBoard) _output_get)
  (Default|UpdateRoundTime (Variables|Default|GetScoreboard2) _output_get)
  (Utilities|Time|SetTimerbyFunctionName 0 "RoundCountdown" 1.0 true))

(event Custom|Update%20Scores
  (params (Player :type Boolean))
  (bind _scoreboard2 (Variables|Default|GetScoreboard2))
  (bind _scoreboard (Variables|Default|GetScoreBoard))
  ;[1 1 1] Updat Player Score On Fall
  (if Player
    (bind _output_get (Variables|Default|SetP1Score (+ (Variables|Default|GetP1Score) 1)))
    (Default|UpdateScore _scoreboard false _output_get)
    (Default|UpdateScore _scoreboard2 false _output_get)
    (else
      (bind _output_get_2 (Variables|Default|SetP2Score (+ (Variables|Default|GetP2Score) 1)))
      (Default|UpdateScore _scoreboard true _output_get_2)
      (Default|UpdateScore _scoreboard2 true _output_get_2))))

(event Custom|Begin%20Match
  ;[1 1 1] Setup New Match
  (Variables|Default|SetRoundTime 300)
  (Variables|Default|SetP1Score 0)
  (Variables|Default|SetP2Score 0)
  (Default|Restart (Variables|Default|GetScoreBoard))
  (Default|Restart (Variables|Default|GetScoreboard2))
  (CallFunction|BeginROund))

(event Custom|RoundCountdown
  ;[1 1 1] Round Timer
  (bind _output_get (Variables|Default|SetRoundTime (- (Variables|Default|GetRoundTime) 1)))
  (Default|UpdateRoundTime (Variables|Default|GetScoreBoard) _output_get)
  (Default|UpdateRoundTime (Variables|Default|GetScoreboard2) _output_get))

(event Custom|PlayerFell
  (params (PlayerChar :type TR%20Player%20Character%20Object%20Reference))
  ;[1 1 1] Player Fell Down
  (if (== PlayerChar (Variables|Default|GetPlayer1Char))
    (Development|PrintString "Player 1 Fell!")
    (CallFunction|UpdateScores false)
    (CallFunction|Teleport)
    (CallFunction|BeginROund)
    (else
      (Development|PrintString "Player 2 Fell!")
      (CallFunction|UpdateScores true)
      (CallFunction|Teleport)
      (CallFunction|BeginROund))))

(event Custom|PlayerHit
  (params (Player :type TR%20Player%20Character%20Object%20Reference))
  ;[1 1 1] Player Hit By Disk (for debug)
)

(event EventPostLogin
  (params (NewPlayer :type Player%20Controller%20Object%20Reference))
  ;[1 1 1] After Player Logon
  (bind _astr_player_state (Utilities|Casting|CastToTR_PlayerState (Variables|/Script/Engine.Controller|GetPlayerState NewPlayer)))
  (Variables|/Game/TR/Blueprints/TR_PlayerState.TR_PlayerState_C|SetPlayerNumber _astr_player_state (Utilities|Array|Length (Variables|/Script/Engine.GameState|GetPlayerArray (Game|GetGameState))))
  (bind _astr_player_controller (Utilities|Casting|CastToTR_PlayerController NewPlayer))
  (Default|ClientPostLogon _astr_player_controller)
  (if (Variables|Default|GetFull)
    (bind _output_get (Variables|Default|SetPlayerC2 _astr_player_controller))
    (bind _astr_player_character (Utilities|Casting|CastToTR_PlayerCharacter (Pawn|GetControlledPawn _astr_player_controller)))
    (Variables|Default|SetPlayer2Char _astr_player_character)
    (Development|PrintString (Utilities|String|Append (Utilities|GetDisplayName _output_get) " Has Joined the Server") true true "(R=0.000000,G=0.660000,B=1.000000,A=1.000000)" 2e+01)
    (else
      (Variables|Default|SetFull true)
      (bind _output_get_2 (Variables|Default|SetPlayerC1 _astr_player_controller))
      (bind _astr_player_character_2 (Utilities|Casting|CastToTR_PlayerCharacter (Pawn|GetControlledPawn _astr_player_controller)))
      (Variables|Default|SetPlayer1Char _astr_player_character_2)
      (Development|PrintString (Utilities|String|Append (Utilities|GetDisplayName _output_get_2) " Has Joined the Server") true true "(R=0.000000,G=0.660000,B=1.000000,A=1.000000)" 2e+01))))

(fn ConstructionScript)

(fn StartGame
  (Variables|Default|SetGameInPlay true)
  (Variables|Default|SetPlayer1Ready false)
  (Variables|Default|SetPlayer2Ready false)
  (if (Variables|Default|GetFirstGame)
    (Variables|Default|SetFirstGame false)
    (CallFunction|Teleport)
    (bind _returnvalue (Game|SpawnActorfromClass "/Game/TR/Blueprints/TR_GameStatus.TR_GameStatus_C" (Math|Transform|MakeTransform "-530.000000,-290.000000,530.000000" "0.000000,180.000000,0.000000") "Undefined" (Variables|Default|GetPlayer1Char) 0))
    (Variables|Default|SetScoreBoard _returnvalue)
    (bind _returnvalue_2 (Game|SpawnActorfromClass "/Game/TR/Blueprints/TR_GameStatus.TR_GameStatus_C" (Math|Transform|MakeTransform "-530.000000,-290.000000,530.000000") "Undefined" (Variables|Default|GetPlayer2Char) 0))
    (Variables|Default|SetScoreboard2 _returnvalue_2)
    (CallFunction|BeginMatch)
    (else
      (CallFunction|Teleport)
      (CallFunction|BeginMatch))))

(fn Teleport
  (bind _playerc2 (Variables|Default|GetPlayerC2))
  (bind _returnvalue (Pawn|GetControlledPawn _playerc2))
  (Transformation|SetActorTransform (Pawn|GetControlledPawn (Variables|Default|GetPlayerC1)) (Math|Transform|MakeTransform "-2010.000000,-70.000000,1000.000000"))
  (Transformation|Teleport _returnvalue "1200.000000,-70.000000,1750.000000" "0, 0, 0")
  (Transformation|SetActorTransform _returnvalue (Math|Transform|MakeTransform "1200.000000,-70.000000,1000.000000")))

(fn OnRepRounds
  (bind _rounds (Variables|Default|GetRounds))
  (if (== _rounds 10)
    (Development|PrintString "10 Rounds Reached, Restarting Game!" true true "(R=0.000000,G=0.660000,B=1.000000,A=1.000000)" 2e+01)
    (CallFunction|RestartEntireGame)
    (else
      (Development|PrintString (Utilities|String|Append "Round:" (Utilities|String|ToString(Integer) _rounds)) true true "(R=0.000000,G=0.660000,B=1.000000,A=1.000000)" 2e+01))))

(fn RestartEntireGame
  (bind _playerc1 (Variables|Default|GetPlayerC1))
  (bind _playerc2 (Variables|Default|GetPlayerC2))
  (bind _returnvalue (Pawn|GetControlledPawn _playerc1))
  (bind _returnvalue_2 (Pawn|GetControlledPawn _playerc2))
  (Variables|Default|SetGameInPlay false)
  (Transformation|SetActorTransform _returnvalue (Math|Transform|MakeTransform "1500.000000,-70.000000,3000.000000"))
  (Transformation|Teleport _returnvalue "1000.000000,-70.000000,3000.000000" "0, 0, 0")
  (Transformation|SetActorTransform _returnvalue_2 (Math|Transform|MakeTransform "1200.000000,-70.000000,1750.000000"))
  (Transformation|Teleport _returnvalue_2 "1000.000000,-70.000000,3000.000000" "0, 0, 0")
  (Variables|Default|SetRounds 0))

(fn P1Ready
  (if (Variables|Default|GetPlayer2Ready)
    (Development|PrintString "Both Players are Ready! Play starting!")
    (CallFunction|StartGame)
    (else
      (Development|PrintString "Player 1 is Ready!"))))

(fn P2Ready
  (if (Variables|Default|GetPlayer1Ready)
    (Development|PrintString "Both Players are Ready! Play starting!")
    (CallFunction|StartGame)
    (else
      (Development|PrintString "Player 2 is Ready!"))))

(fn P1RestartCheck
  (Variables|Default|SetP1Restart true)
  (if (Variables|Default|GetP2Restart)
    (Development|PrintString "Both Players Agree to Restart" true true "(R=0.000000,G=0.660000,B=1.000000,A=1.000000)" 2e+01)
    (Variables|Default|SetP1Restart false)
    (Variables|Default|SetP2Restart false)
    (CallFunction|RestartEntireGame)
    (else
      (Development|PrintString "Player 1 Wants to Restart  the Game" true true "(R=0.000000,G=0.660000,B=1.000000,A=1.000000)" 2e+01))))

(fn P2RestartCheck
  (Variables|Default|SetP2Restart true)
  (if (Variables|Default|GetP1Restart)
    (Development|PrintString "Both Players Agree to Restart the game" true true "(R=0.000000,G=0.660000,B=1.000000,A=1.000000)" 2e+01)
    (Variables|Default|SetP1Restart false :!label _label)
    (Variables|Default|SetP2Restart false)
    (CallFunction|RestartEntireGame)
    (goto _label)
    (else
      (Development|PrintString "Player 2 Wants to restart the Game" true true "(R=0.000000,G=0.660000,B=1.000000,A=1.000000)" 2e+01))))