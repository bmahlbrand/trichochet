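; TR_GameStatus is a status display Blueprint that shows both players' scores and the current round time.
; UpdateScore uses a boolean to write to either the P1 (false) or P2 (true) score text, and UpdateRoundTime writes the time text.
; Restart resets the display through both events, zeroing the scores and restoring the starting time.
; It only displays values passed to it, with no Tick logic or stored game state.
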(event Custom|UpdateScore
  (params (Player :type Boolean) (Score :type Integer))
  (if Player
    (Rendering|Components|TextRender|SetText (Variables|Default|GetcurrentP2Score) (Utilities|Text|ToText(Integer) Score))
    (else
      (Rendering|Components|TextRender|SetText (Variables|Default|GetcurrentP1Score) (Utilities|Text|ToText(Integer) Score)))))

(event Custom|UpdateRoundTime
  (params (CurrentTime :type Integer))
  (Rendering|Components|TextRender|SetText (Variables|Default|GetCurrentTime) (Utilities|Text|ToText(Integer) CurrentTime)))

(event Custom|Restart
  (CallFunction|UpdateScore false)
  (CallFunction|UpdateScore true)
  (CallFunction|UpdateRoundTime 300))

(event EventBeginPlay)

(event EventActorBeginOverlap
  (params (OtherActor :type Actor%20Object%20Reference)))

(event EventTick
  (params (DeltaSeconds :type Float%20%28single-precision%29)))

(fn ConstructionScript)