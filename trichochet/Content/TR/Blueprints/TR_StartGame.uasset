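; TR_StartGame is a trigger actor that marks a player as ready when their character overlaps its Box component.
; The overlap resolves the TR_PlayerCharacter's controller and compares it with PlayerC1 on TR_GameMode to identify the player.
; It then sets that player's ready flag on the game mode and calls P1Ready or P2Ready, treating any controller other than PlayerC1 as player two.
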(event OnComponentBeginOverlap(Box)
  (params (OtherActor :type Actor%20Object%20Reference) (OtherComp :type Primitive%20Component%20Object%20Reference) (OtherBodyIndex :type Integer) (bFromSweep :type Boolean) (SweepResult :type Hit%20Result%20Structure%20%28by%20ref%29))
  (bind _astr_game_mode (Utilities|Casting|CastToTR_GameMode (Game|GetGameMode)))
  (bind _astr_player_character (Utilities|Casting|CastToTR_PlayerCharacter OtherActor))
  (bind _astr_player_controller (Utilities|Casting|CastToTR_PlayerController (Pawn|GetController _astr_player_character)))
  (if (== (Variables|/Game/TR/Blueprints/TR_GameMode.TR_GameMode_C|GetPlayerC1 _astr_game_mode) _astr_player_controller)
    (Variables|/Game/TR/Blueprints/TR_GameMode.TR_GameMode_C|SetPlayer1Ready _astr_game_mode true)
    (Default|P1Ready _astr_game_mode)
    (else
      (Variables|/Game/TR/Blueprints/TR_GameMode.TR_GameMode_C|SetPlayer2Ready _astr_game_mode true)
      (Default|P2Ready _astr_game_mode))))

(event EventBeginPlay)

(fn ConstructionScript)