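; TR_Music is a placeable actor that switches the player's music by zone.
; It has four overlap components named Brut, Tron, Whip and Epic.
; When a TR_PlayerCharacter begins overlapping one, the actor calls that character's Music function with that zone's track index.
; The character handles the switch itself; the actor has no end-overlap, Tick or construction logic.
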(event OnComponentBeginOverlap(Epic)
  (params (OtherActor :type Actor%20Object%20Reference) (OtherComp :type Primitive%20Component%20Object%20Reference) (OtherBodyIndex :type Integer) (bFromSweep :type Boolean) (SweepResult :type Hit%20Result%20Structure%20%28by%20ref%29))
  (bind _astr_player_character (Utilities|Casting|CastToTR_PlayerCharacter OtherActor))
  (Default|Music _astr_player_character 3))

(event OnComponentBeginOverlap(Brut)
  (params (OtherActor :type Actor%20Object%20Reference) (OtherComp :type Primitive%20Component%20Object%20Reference) (OtherBodyIndex :type Integer) (bFromSweep :type Boolean) (SweepResult :type Hit%20Result%20Structure%20%28by%20ref%29))
  (bind _astr_player_character (Utilities|Casting|CastToTR_PlayerCharacter OtherActor))
  (Default|Music _astr_player_character 1))

(event OnComponentBeginOverlap(Tron)
  (params (OtherActor :type Actor%20Object%20Reference) (OtherComp :type Primitive%20Component%20Object%20Reference) (OtherBodyIndex :type Integer) (bFromSweep :type Boolean) (SweepResult :type Hit%20Result%20Structure%20%28by%20ref%29))
  (bind _astr_player_character (Utilities|Casting|CastToTR_PlayerCharacter OtherActor))
  (Default|Music _astr_player_character))

(event OnComponentBeginOverlap(Whip)
  (params (OtherActor :type Actor%20Object%20Reference) (OtherComp :type Primitive%20Component%20Object%20Reference) (OtherBodyIndex :type Integer) (bFromSweep :type Boolean) (SweepResult :type Hit%20Result%20Structure%20%28by%20ref%29))
  (bind _astr_player_character (Utilities|Casting|CastToTR_PlayerCharacter OtherActor))
  (Default|Music _astr_player_character 2))

(event EventBeginPlay)

(event EventActorBeginOverlap
  (params (OtherActor :type Actor%20Object%20Reference)))

(event EventTick
  (params (DeltaSeconds :type Float%20%28single-precision%29)))

(fn ConstructionScript)