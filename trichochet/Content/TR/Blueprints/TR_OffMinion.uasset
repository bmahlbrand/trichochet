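; Stationary ranged minion that fires a repeating volley of TR_Projectile shots from above its origin.
; BeginPlay starts a looping timer that calls Shoot, which plays the shooting animation and spawns three projectiles separated by delays: one straight, then one angled to each side.
; The actor's own rotation selects between two opposite firing directions, with the order of the angled shots mirrored between them.
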(event Custom|Shoot
  (bind _returnvalue (Transformation|GetActorLocation))
  (bind _returnvalue_2 (Transformation|GetActorLocation))
  (bind _skeletalmesh (Variables|Default|GetSkeletalMesh))
  (bind _returnvalue_3 (+ _returnvalue "0, 0,300.000000" "0.000000,0.000000,0.000000"))
  (bind _returnvalue_4 (+ _returnvalue_2 "0, 0,300.000000" "0.000000,0.000000,0.000000"))
  (Components|Animation|SetAnimation _skeletalmesh "/Game/MixamoAnimPack/Mixamo_Alpha/Anims/mixamo_Shooting.mixamo_Shooting")
  (Audio|Components|Audio|Play _skeletalmesh false)
  (if (Math|Rotator|Equal(Rotator) (Transformation|GetActorRotation) "0,90.000000, 0" 0.0001)
    (bind _output_get (Variables|Default|SetOffset "0,180.000000, 0"))
    (Game|SpawnActorfromClass "/Game/TR/Blueprints/TR_Projectile.TR_Projectile_C" (Math|Transform|MakeTransform _returnvalue_4 _output_get) "AlwaysSpawn" 0 0) ; Spawn projectile
    (Utilities|FlowControl|Delay 1.5)
    (Game|SpawnActorfromClass "/Game/TR/Blueprints/TR_Projectile.TR_Projectile_C" (Math|Transform|MakeTransform _returnvalue_4 (Math|Rotator|CombineRotators (Variables|Default|GetOffset) "0,20.000000, 0")) "AlwaysSpawn" 0 0) ; Spawn projectile
    (Utilities|FlowControl|Delay 2.0)
    (Game|SpawnActorfromClass "/Game/TR/Blueprints/TR_Projectile.TR_Projectile_C" (Math|Transform|MakeTransform _returnvalue_4 (Math|Rotator|CombineRotators (Variables|Default|GetOffset) "0,-20.000000, 0")) "AlwaysSpawn" 0 0) ; Spawn projectile
    (else
      (bind _output_get_2 (Variables|Default|SetOffset "0,0.000000, 0"))
      (Game|SpawnActorfromClass "/Game/TR/Blueprints/TR_Projectile.TR_Projectile_C" (Math|Transform|MakeTransform _returnvalue_3 _output_get_2) "AlwaysSpawn" 0 0) ; Spawn projectile
      (Utilities|FlowControl|Delay 1.5)
      (Game|SpawnActorfromClass "/Game/TR/Blueprints/TR_Projectile.TR_Projectile_C" (Math|Transform|MakeTransform _returnvalue_3 (Math|Rotator|CombineRotators (Variables|Default|GetOffset) "0,-20.000000, 0")) "AlwaysSpawn" 0 0) ; Spawn projectile
      (Utilities|FlowControl|Delay 2.0)
      (Game|SpawnActorfromClass "/Game/TR/Blueprints/TR_Projectile.TR_Projectile_C" (Math|Transform|MakeTransform _returnvalue_3 (Math|Rotator|CombineRotators (Variables|Default|GetOffset) "0,20.000000, 0")) "AlwaysSpawn" 0 0) ; Spawn projectile
    )))

(event Custom|Shooter
  (Utilities|Time|SetTimerbyFunctionName 0 "Shoot" 4.0 true))

(event EventBeginPlay
  (CallFunction|Shooter))

(fn ConstructionScript)